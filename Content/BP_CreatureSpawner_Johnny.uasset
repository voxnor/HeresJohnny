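; Creature spawner for Johnny that permanently stops once its creature is destroyed, tracked by an IsDefeated flag.
; On BeginPlay, unless defeated, a looping timer polls the creature list until one exists, then binds to the first one's OnDestroyed and stops polling.
; That event sets IsDefeated, clears the creature class and destroys the remaining spawned creatures.
; ShouldSave always returns true, opting the spawner into saving.
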(event `self.ReceiveBeginPlay`
  (`parent.ReceiveBeginPlay`)
  (if (not (`self.bIsDefeated`))
    (bind _returnvalue (`KismetSystemLibrary.K2_SetTimerDelegate` (delegate `PollForSpawn`) 2.0 true))
    (set `self.PollingTimerHandle` _returnvalue)))

(event `PollForSpawn`
  (bind _returnvalue (`self.GetCreatures`))
  (if (`KismetArrayLibrary.Array_IsNotEmpty` _returnvalue)
    (add `self.OnDestroyed` (`|GetArrayItem` _returnvalue) (delegate `JohnnyDeath`))
    (`KismetSystemLibrary.K2_ClearAndInvalidateTimerHandle` (`self.PollingTimerHandle`))))

(event `JohnnyDeath` :!signature `self.OnDestroyed`
  (params (DestroyedActor :type "Actor Object Reference"))
  (set `self.bIsDefeated` true)
  (set `self.mCreatureClass` null)
  (`self.DestroyChildren`))

(fn `DestroyChildren`
  (for _array_element (`self.GetCreatures`)
    (`self.K2_DestroyActor` _array_element)))

(fn `ShouldSave`
  (returns (ReturnValue :type Boolean))
  (return true))

(fn `UserConstructionScript`)

(fn `UserConstructionScript_0`)